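; BP_Battery is a pickup actor that gives the first-person character a spare battery.
; On BeginPlay it caches a reference to player 0's BP_FirstPersonCharacter.
; When that character overlaps its Sphere while below the spare battery limit, it sets the character's picked-up flag and increments the spare count.
; It then plays a collect sound at the character's location and destroys itself.
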(event OnComponentBeginOverlap(Sphere)
  (params (OverlappedComponent :type Primitive%20Component%20Object%20Reference) (OtherActor :type Actor%20Object%20Reference) (OtherComp :type Primitive%20Component%20Object%20Reference) (OtherBodyIndex :type Integer) (bFromSweep :type Boolean) (SweepResult :type Hit%20Result%20Structure%20%28by%20ref%29))
  (bind _as_bp_first_person_character (Variables|Default|GetAs%20BP%20First%20Person%20Character))
  (bind _as_bp_first_person_character_2 (Variables|Default|GetAs%20BP%20First%20Person%20Character))
  ;[0.15 0.15 0.15 0.5] Pick Up Battery
  (if (and (== OtherActor _as_bp_first_person_character) (< (Variables|/Game/StarterContent/FirstPerson/Blueprints/BP_FirstPersonCharacter.BP_FirstPersonCharacter_C|GetSpareBatteryAmount _as_bp_first_person_character) (Variables|/Game/StarterContent/FirstPerson/Blueprints/BP_FirstPersonCharacter.BP_FirstPersonCharacter_C|GetSpareBatteryMax _as_bp_first_person_character)))
    (Variables|/Game/StarterContent/FirstPerson/Blueprints/BP_FirstPersonCharacter.BP_FirstPersonCharacter_C|SetBatteryPickedUp (Variables|Default|GetAs%20BP%20First%20Person%20Character) true)
    (Variables|/Game/StarterContent/FirstPerson/Blueprints/BP_FirstPersonCharacter.BP_FirstPersonCharacter_C|SetSpareBatteryAmount _as_bp_first_person_character_2 (+ (Variables|/Game/StarterContent/FirstPerson/Blueprints/BP_FirstPersonCharacter.BP_FirstPersonCharacter_C|GetSpareBatteryAmount _as_bp_first_person_character) 1))
    (Audio|PlaySoundatLocation "/Game/MyContent/Audio/MP3_Key_Collect.MP3_Key_Collect" (Transformation|GetActorLocation _as_bp_first_person_character_2) "0, 0, 0" 1.0 1.0 0.0 0 0 0 0)
    (Actor|DestroyActor)))

(event EventBeginPlay
  ;[0.15 0.15 0.15 0.5] Setup
  (bind _asbp_first_person_character (Utilities|Casting|CastToBP_FirstPersonCharacter (Game|GetPlayerCharacter 0)))
  (Variables|Default|SetAs%20BP%20First%20Person%20Character _asbp_first_person_character))

(event Collision|EventActorBeginOverlap
  (params (OtherActor :type Actor%20Object%20Reference)))

(event EventTick
  (params (DeltaSeconds :type Float%20%28single-precision%29)))

(fn ConstructionScript)